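; BP_MazeGenerator is an early-stage maze generator that lays out a flat grid of floor tiles, with no maze-carving logic yet.
; The Construction Script derives cell size from the floor mesh's X extent, then records each GridSizeX by GridSizeY cell in TilesList with its row, column and cleared flags.
; Each entry becomes a local-space instance on a Hierarchical Instanced Static Mesh, while BeginPlay is empty.
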(event EventBeginPlay)

(fn ConstructionScript
  (bind _floormesh (Variables|Default|GetFloorMesh))
  (bind _returnvalue (StaticMesh|GetBoundingBox _floormesh))
  (Components|StaticMesh|SetStaticMesh (Variables|Default|GetHISMFloor) (Variables|Default|GetFloorMesh))
  (Variables|Default|SetCellSize (.X (Math|Vector|BreakVector (- (.max _returnvalue) (.min _returnvalue)))))
  (for _index (range 0 (- (Variables|Default|GetGridSizeX) 1))
    (for _index_2 (range 0 (- (Variables|Default|GetGridSizeY) 1))
      (bind _returnvalue_2 (Utilities|Array|Add (Variables|Default|GetTilesList) (Utilities|Struct|MakeMazeStructure "0.000000,0.000000,0.000000|0.000000,0.000000,0.000000|1.000000,1.000000,1.000000" false false 0 "0.000000,0.000000,0.000000" _index_2 _index false false false false)))
      (Components|InstancedStaticMesh|AddInstance (Variables|Default|GetHISMFloor) (Math|Transform|MakeTransform (Math|Vector|MakeVector (* (.Col (Utilities|Struct|BreakMazeStructure (Utilities|Array|Get(acopy) (Variables|Default|GetTilesList) _returnvalue_2))) (Variables|Default|GetCellSize)) (* (Variables|Default|GetCellSize) (.Row (Utilities|Struct|BreakMazeStructure (Utilities|Array|Get(acopy) (Variables|Default|GetTilesList) _returnvalue_2)))) 0.0)) false))))